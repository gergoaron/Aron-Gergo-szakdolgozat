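; AI controller that plays the opponent's side in a turn-based card game.
; On BeginPlay it caches the game state, mode and card placement, builds a shuffled deck from the BlueDeck data table row, and creates the opponent HUD.
; Each turn it draws two cards into the HUD hand by DT_Cards lookup, places the first card in hand without any selection logic, then passes the turn through the game state, using delays for pacing.
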(event `LoadDeck`
  (bind _deck (`self.Deck`))
  (bind _returnvalue (`|GetDataTableRow` "/Game/CardUI/DT_Default_Deck.DT_Default_Deck" "BlueDeck")
    (:`then`
      (bind _output_get (set `self.StartingDeck` _returnvalue))
      (for _array_element (`.Cards_6_49B140444B2EBD7D22C971A283AB63AF` (break `/Game/CardUI/S_Deck` _output_get))
        (bind (_cardname _quantity) (break `/Game/CardUI/S_Deck_Row` _array_element))
        (for _ (range 1 (+ _quantity 1))
          (`KismetArrayLibrary.Array_Add` _deck _cardname)))
      (`KismetArrayLibrary.Array_Shuffle` _deck))))

(event `self.ReceiveBeginPlay`
  (bind _asbp_card_game_state (cast `/Game/CardUI/BP_CardGameState` (`GameplayStatics.GetGameState`)))
  (set `self.GameState` _asbp_card_game_state)
  (bind _asbp_card_game_mode (cast `/Game/CardUI/BP_CardGameMode` (`GameplayStatics.GetGameMode`)))
  (bind _output_get (set `self.GameMode` _asbp_card_game_mode))
  (set `self.OpponentCardPlacement` (`/Game/CardUI/BP_CardGameMode.OpponentCardPlacement` _output_get))
  (`self.LoadDeck`)
  (bind _returnvalue (`|CreateWidget` "/Game/CardUI/W_OpponentHUD.W_OpponentHUD_C"))
  (bind _output_get_2 (set `self.OpponentHUD` _returnvalue))
  (`UserWidget.AddToViewport` _output_get_2 0))

(event `ChangeTurn`
  (bind _asbp_card_game_state (cast `/Game/CardUI/BP_CardGameState` (`GameplayStatics.GetGameState`)))
  (if (not (`/Game/CardUI/BP_CardGameState.IsPlayersTurn` _asbp_card_game_state))
    (`/Game/CardUI/BP_CardGameState.ChangeTurn` _asbp_card_game_state)))

(event `/Game/CardUI/BPI_CardController.StartTurn`
  (`self.DrawCard`)
  (`self.DrawCard`)
  (`KismetSystemLibrary.Delay` 1.0)
  (`self.Play Card`)
  (`KismetSystemLibrary.Delay` 2.0)
  (`self.ChangeTurn`))

(event `/Game/CardUI/BPI_CardController.EndTurn`)

(event `Play Card`
  (bind _output (`|GetArrayItem` (`/Game/CardUI/W_OpponentHand.CardWidgetRef` (`/Game/CardUI/W_OpponentHUD.OpponentHand` (`self.OpponentHUD`)))))
  (`self.PlaceCard` (`/Game/CardUI/W_Card.CardInfo` _output))
  (`/Game/CardUI/W_OpponentHand.RemoveCard` (`/Game/CardUI/W_OpponentHUD.OpponentHand` (`self.OpponentHUD`)) _output))

(fn `DrawCard`
  (if (> (`KismetArrayLibrary.Array_Length` (`self.Deck`)) 0)
    (bind _returnvalue (`|GetDataTableRow` "/Game/CardUI/DT_Cards.DT_Cards" (`|GetArrayItem` (`self.Deck`)))
      (:`then`
        (`KismetArrayLibrary.Array_Remove` (`self.Deck`))
        (if (`KismetTextLibrary.TextIsEmpty` (`.CardName_3_EF5C332F4601C99F45A7348175DE8CEC` (break `/Game/CardUI/S_CardInfo` _returnvalue)))
          (`KismetSystemLibrary.PrintString` "Deck Empty")
          (else
            (message `/Game/CardUI/BPI_AddCard.AddCard` (`/Game/CardUI/W_OpponentHUD.OpponentHand` (`self.OpponentHUD`)) _returnvalue))))
      (:`RowNotFound`
        (`KismetSystemLibrary.PrintString` "Row not Found")))
    (else
      (return))))

(fn `PlaceCard`
  (params (CardInfo :type "/Game/CardUI/S_CardInfo Structure"))
  (`/Game/CardUI/BP_CardPlacement.PlaceCard` (`self.OpponentCardPlacement`) CardInfo self)
  (return))

(fn `UserConstructionScript`)