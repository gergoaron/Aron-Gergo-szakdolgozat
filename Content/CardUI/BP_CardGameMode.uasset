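; Game mode for a player-versus-AI card game, setting up the board, both participants and the game-over screen.
; BeginPlay spawns a card placement area and hero for each side.
; PostLogin spawns the AI controller, initializes both player states and starts the game state; GameStart fires without waiting for the delayed BeginGame inside the loop.
; GameOver shows a win/loss widget by comparing the dead hero's owner to the first controller's name.
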(event `self.K2_PostLogin`
  (params (NewPlayer :type "PlayerController Object Reference"))
  (`KismetArrayLibrary.Array_AddUnique` (`self.PlayerControllers`) NewPlayer)
  (bind _asbp_card_player_state (cast `/Game/CardUI/BP_CardPlayerState` (`Controller.PlayerState` NewPlayer)))
  (`KismetArrayLibrary.Array_AddUnique` (`self.PlayerStates`) _asbp_card_player_state)
  (bind _returnvalue (`|SpawnActorFromClass` "/Game/CardUI/BP_CardAIController.BP_CardAIController_C" (`KismetMathLibrary.MakeTransform` (0.0 0.0 0.0)) "Undefined" "MultiplyWithRoot" null null))
  (`KismetArrayLibrary.Array_AddUnique` (`self.PlayerControllers`) _returnvalue)
  (bind _asbp_card_player_state_2 (cast `/Game/CardUI/BP_CardPlayerState` (`Controller.PlayerState` _returnvalue))
    (:`then`
      (`KismetArrayLibrary.Array_AddUnique` (`self.PlayerStates`) _asbp_card_player_state_2))
    (:`CastFailed`
      _))
  (bind _asbp_card_game_state (cast `/Game/CardUI/BP_CardGameState` (`GameplayStatics.GetGameState`)))
  (bind _output_get (set `self.GameStatew` _asbp_card_game_state))
  (for (_array_element _array_index) (`self.PlayerStates`)
    (`/Game/CardUI/BP_CardPlayerState.Init` _array_element (`self.MaxHealth`) (`self.MaxMana`) (`self.MaxCardsInHand`) (`|GetArrayItem` (`self.PlayerControllers`) _array_index))
    (`KismetSystemLibrary.Delay` 1.0)
    (`/Game/CardUI/BP_CardGameState.BeginGame` (`self.GameStatew`)))
  (`/Game/CardUI/BP_CardGameState.GameStart` _output_get))

(event `self.ReceiveBeginPlay`
  (bind _returnvalue (`|SpawnActorFromClass` "/Game/CardUI/BP_CardPlacement.BP_CardPlacement_C" (`KismetMathLibrary.MakeTransform` (200.0 0.0 0.0)) "Undefined" "MultiplyWithRoot" null null))
  (set `self.PlayerCardPlacement` _returnvalue)
  (bind _returnvalue_2 (`|SpawnActorFromClass` "/Game/CardUI/BP_CardPlacement.BP_CardPlacement_C" (`KismetMathLibrary.MakeTransform` (-200.0 0.0 0.0)) "Undefined" "MultiplyWithRoot" null null))
  (set `self.OpponentCardPlacement` _returnvalue_2)
  (bind _returnvalue_3 (`|SpawnActorFromClass` "/Game/CardUI/BP_HeroInstance.BP_HeroInstance_C" (`KismetMathLibrary.MakeTransform` (200.0 900.0 1.0)) "Undefined" "MultiplyWithRoot" null null 10 null))
  (set `self.PlayerHero` _returnvalue_3)
  (bind _returnvalue_4 (`|SpawnActorFromClass` "/Game/CardUI/BP_HeroInstance.BP_HeroInstance_C" (`KismetMathLibrary.MakeTransform` (-200.0 900.0 1.0)) "Undefined" "MultiplyWithRoot" null null 10 null))
  (set `self.OpponentHero` _returnvalue_4))

(event `GameOver`
  (params (DeadHeroOwner :type String))
  (bind _returnvalue (`|CreateWidget` "/Game/CardUI/Widgets/W_GameOver.W_GameOver_C" null (not (`KismetStringLibrary.EqualEqual_StrStr` DeadHeroOwner (`KismetSystemLibrary.GetObjectName` (`|GetArrayItem` (`self.PlayerControllers`)))))))
  (`UserWidget.AddToViewport` _returnvalue 0))

(fn `UserConstructionScript`)