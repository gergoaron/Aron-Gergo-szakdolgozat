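; Player controller for a turn-based card battler, handling the player's deck, HUD, mana and board input.
; BeginPlay creates the HUD and builds a shuffled deck from a data table; each turn start refreshes mana and attacks, then draws a card.
; PlaceCard validates turn, placement box, capacity and mana.
; Mouse drag opens a gated Tick cursor trace for targets; release sends card or hero attacks to the game state.
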(event `LoadDeck`
  (bind _deck (`self.Deck`))
  (bind _returnvalue (`|GetDataTableRow` "/Game/CardUI/DT_Default_Deck.DT_Default_Deck" "BlueDeck")
    (:`then`
      (bind _output_get (set `self.StartingDeck` _returnvalue))
      (for _array_element (`.Cards_6_49B140444B2EBD7D22C971A283AB63AF` (break `/Game/CardUI/S_Deck` _output_get))
        (bind (_cardname _quantity) (break `/Game/CardUI/S_Deck_Row` _array_element))
        (for _ (range 1 (+ _quantity 1))
          (`KismetArrayLibrary.Array_Add` _deck _cardname)))
      (`KismetArrayLibrary.Array_Shuffle` _deck))))

(event `self.ReceiveBeginPlay`
  (bind _returnvalue (`|CreateWidget` "/Game/CardUI/W_CardHUD.W_CardHUD_C" self))
  (bind _output_get (set `self.CardHUD` _returnvalue))
  (`UserWidget.AddToViewport` _returnvalue 0)
  (`UserWidget.AddToViewport` _output_get 0)
  (bind _asbp_card_game_mode (cast `/Game/CardUI/BP_CardGameMode` (`GameplayStatics.GetGameMode`)))
  (set `self.PlayerCardPlacement` (`/Game/CardUI/BP_CardGameMode.PlayerCardPlacement` _asbp_card_game_mode))
  (bind _output_get_2 (set `self.Hero` (`/Game/CardUI/BP_CardGameMode.PlayerHero` _asbp_card_game_mode)))
  (`self.SetOwner` _output_get_2 self)
  (set `self.bShowMouseCursor` true)
  (bind _asbp_card_game_state (cast `/Game/CardUI/BP_CardGameState` (`GameplayStatics.GetGameState`)))
  (set `self.GameState` _asbp_card_game_state)
  (bind _asbp_card_player_state (cast `/Game/CardUI/BP_CardPlayerState` (`GameplayStatics.GetPlayerState` 0)))
  (set `self.CardPlayerState` _asbp_card_player_state)
  (`self.LoadDeck`))

(event `ChangeTurn`
  (bind _asbp_card_game_state (cast `/Game/CardUI/BP_CardGameState` (`GameplayStatics.GetGameState`)))
  (if (`/Game/CardUI/BP_CardGameState.IsPlayersTurn` _asbp_card_game_state)
    (`/Game/CardUI/BP_CardGameState.ChangeTurn` _asbp_card_game_state)))

(event `/Game/CardUI/BPI_CardController.EndTurn`
  (set `self.IsPlayersTurn` false))

(event `self.ReceiveTick`
  (params (DeltaSeconds :type "Float (single-precision)"))
  (bind (_bblockinghit _binitialoverlap _time _distance _location _impactpoint _normal _impactnormal _physmat _hitactor) (`GameplayStatics.BreakHitResult` (`self.GetHitResultUnderCursorByChannel` "TraceTypeQuery1")))
  (bind _returnvalue (`GameplayStatics.GetObjectClass` _hitactor))
  (`/Engine/EditorBlueprintResources/StandardMacros.Gate` true :!label _label
    (:`Exit`
      (`/Engine/EditorBlueprintResources/StandardMacros.IsValid` _hitactor
        (:`Is Valid`
          (if (== _returnvalue "/Game/CardUI/BP_CardInstance.BP_CardInstance_C")
            (bind _asbp_card_instance (cast `/Game/CardUI/BP_CardInstance` _hitactor))
            (bind _returnvalue_2 (`KismetSystemLibrary.GetObjectName` _asbp_card_instance))
            (if (`KismetStringLibrary.EqualEqual_StrStr` _returnvalue_2 (`KismetSystemLibrary.GetObjectName` (`self.DraggedCard`)))
              _
              (elif (not (`KismetStringLibrary.EqualEqual_StrStr` _returnvalue_2 (`KismetSystemLibrary.GetObjectName` (`self.TargetedCard`))))
                (set `self.TargetedCard` _asbp_card_instance)))
            (elif (== _returnvalue "/Game/CardUI/BP_HeroInstance.BP_HeroInstance_C")
              (bind _asbp_hero_instance (cast `/Game/CardUI/BP_HeroInstance` _hitactor))
              (set `self.TargetedHero` _asbp_hero_instance))))))))

(event `/Game/CardUI/BPI_CardController.StartTurn`
  (bind _cardplayerstate (`self.CardPlayerState`))
  (set `self.IsPlayersTurn` true)
  (set `/Game/CardUI/BP_CardPlayerState.Mana` (`KismetMathLibrary.Min` (`/Game/CardUI/BP_CardGameState.TurnNumber` (`self.GameState`)) (`/Game/CardUI/BP_CardPlayerState.MaxMana` _cardplayerstate)) _cardplayerstate)
  (for _array_element (`/Game/CardUI/BP_CardPlacement.Cards` (`self.PlayerCardPlacement`))
    (set `/Game/CardUI/BP_CardInstance.AttacksRemaining` (`.AttacksPerRound_36_498B980F48A3C459B2591CA008C11C0B` (break `/Game/CardUI/S_CardInfo` (`/Game/CardUI/BP_CardInstance.CardInfo` _array_element))) _array_element))
  (`self.DrawCard`))

(event `Key|LeftMouseButton`
  (params (Key :type "Key Structure"))
  (bind _returnvalue (`GameplayStatics.GetGameState`))
  (bind (_bblockinghit _binitialoverlap _time _distance _location _impactpoint _normal _impactnormal _physmat _hitactor) (`GameplayStatics.BreakHitResult` (`self.GetHitResultUnderCursorByChannel` "TraceTypeQuery1")))
  (:`Pressed`
    (if (`self.IsPlayersTurn`)
      (set `self.TargetedCard` null)
      (if _bblockinghit
        (`/Engine/EditorBlueprintResources/StandardMacros.IsValid` _hitactor
          (:`Is Valid`
            (if (== (`GameplayStatics.GetObjectClass` _hitactor) "/Game/CardUI/BP_CardInstance.BP_CardInstance_C")
              (bind _asbp_card_instance (cast `/Game/CardUI/BP_CardInstance` _hitactor))
              (if (`/Game/CardUI/BP_CardInstance.CanAttack` _asbp_card_instance)
                (bind _output_get (set `self.DraggedCard` _asbp_card_instance))
                (set `/Game/CardUI/BP_CardInstance.IsSelected` true _output_get)
                (`/Game/CardUI/BP_CardPlacement.UpdateCardPositions` (`self.PlayerCardPlacement`))
                (goto _label :!via `Open`))))))))
  (:`Released`
    (if true
      (`|ExecutionSequence`
        (:`then_0`
          (goto _label :!via `Close`))
        (:`then_1`
          (if (`KismetStringLibrary.EqualEqual_StrStr` (`KismetSystemLibrary.GetObjectName` (`self.DraggedCard`)))
            _
            (elif (`KismetStringLibrary.EqualEqual_StrStr` (`KismetSystemLibrary.GetObjectName` (`self.TargetedCard`)))
              (if (not (`KismetStringLibrary.EqualEqual_StrStr` (`KismetSystemLibrary.GetObjectName` (`self.TargetedHero`))))
                (bind _asbp_card_game_state (cast `/Game/CardUI/BP_CardGameState` _returnvalue))
                (`/Game/CardUI/BP_CardGameState.Attack Hero` _asbp_card_game_state (`self.DraggedCard`) (`self.TargetedHero`)))
              (else
                (bind _asbp_card_game_state_2 (cast `/Game/CardUI/BP_CardGameState` _returnvalue))
                (`/Game/CardUI/BP_CardGameState.AttackCard` _asbp_card_game_state_2 (`self.DraggedCard`) (`self.TargetedCard`))))))
        (:`then_2`
          (if (not (`KismetStringLibrary.EqualEqual_StrStr` (`KismetSystemLibrary.GetObjectName` (`self.DraggedCard`))))
            (set `/Game/CardUI/BP_CardInstance.IsSelected` false (`self.DraggedCard`))
            (`/Game/CardUI/BP_CardPlacement.UpdateCardPositions` (`self.PlayerCardPlacement`)))
          (set `self.TargetedCard` null)
          (set `self.DraggedCard` null)
          (set `self.TargetedHero` null))))))

(fn `DrawCard`
  (if (> (`KismetArrayLibrary.Array_Length` (`self.Deck`)) 0)
    (bind _returnvalue (`|GetDataTableRow` "/Game/CardUI/DT_Cards.DT_Cards" (`|GetArrayItem` (`self.Deck`)))
      (:`then`
        (`KismetArrayLibrary.Array_Remove` (`self.Deck`))
        (if (`KismetTextLibrary.TextIsEmpty` (`.CardName_3_EF5C332F4601C99F45A7348175DE8CEC` (break `/Game/CardUI/S_CardInfo` _returnvalue)))
          (`KismetSystemLibrary.PrintString` "Deck Empty")
          (else
            (message `/Game/CardUI/BPI_AddCard.AddCard` (`/Game/CardUI/W_CardHUD.W_CardHand` (`self.CardHUD`)) _returnvalue))))
      (:`RowNotFound`
        (`KismetSystemLibrary.PrintString` "Row not Found")))
    (else
      (`KismetSystemLibrary.PrintString` "empty")
      (return))))

(fn `IsLocationInPlacement`
  (params (Location :type "Vector Structure"))
  (returns (InPlacement :type Boolean))
  (bind _playercardplacement (`self.PlayerCardPlacement`))
  (bind _playercardplacement_2 (`self.PlayerCardPlacement`))
  (return (and (< (`KismetArrayLibrary.Array_Length` (`/Game/CardUI/BP_CardPlacement.Cards` _playercardplacement_2)) (`/Game/CardUI/BP_CardPlacement.MaximumCards` _playercardplacement_2)) (`KismetMathLibrary.IsPointInBox` Location (`self.K2_GetActorLocation` _playercardplacement) (`BoxComponent.GetScaledBoxExtent` (`/Game/CardUI/BP_CardPlacement.PlacementBox` _playercardplacement))))))

(fn `PlaceCard`
  (params (CardLocation :type "Vector Structure") (CardInfo :type "/Game/CardUI/S_CardInfo Structure"))
  (returns (CardPlaced :type Boolean))
  (bind (_cardname _cardimage _carddescription _backgroundcolor _cardmana) (break `/Game/CardUI/S_CardInfo` CardInfo))
  (bind _cardplayerstate (`self.CardPlayerState`))
  (bind _mana (`/Game/CardUI/BP_CardPlayerState.Mana` _cardplayerstate))
  (if (`self.IsPlayersTurn`)
    (bind _inplacement (`self.IsLocationInPlacement` CardLocation))
    (if _inplacement
      (if (>= _mana _cardmana)
        (bind _output_get (set `/Game/CardUI/BP_CardPlayerState.Mana` (- _mana _cardmana) _cardplayerstate))
        (`KismetSystemLibrary.PrintString` (`KismetStringLibrary.Conv_IntToString` _output_get))
        (`/Game/CardUI/BP_CardPlacement.PlaceCard` (`self.PlayerCardPlacement`) CardInfo self)
        (message `/Game/CardUI/BPI_PlayerUI.UpdatePlayerStatsUI` (`self.CardHUD`) (`self.CardPlayerState`))
        (return true)
        (else
          _))))
  (return false))

(fn `UserConstructionScript`)