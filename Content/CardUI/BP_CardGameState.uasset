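; Game state for a two-sided card game that manages game start, turn order and card attacks.
; BeginGame picks the first side at random and has each controller in the GameMode's list draw a starting hand.
; ChangeTurn alternates start/end turn messages between two controllers, counts full rounds and updates the first controller's HUD.
; Attack rejects same-owner targets, then deals attacker's attack to target and target's health to attacker.
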(event `GameStart`
  (bind _asbp_card_game_mode (cast `/Game/CardUI/BP_CardGameMode` (`GameplayStatics.GetGameMode`)))
  (set `self.GameMode` _asbp_card_game_mode))

(event `ChangeTurn`
  (if (!= (`self.IsPlayersTurn`) (`self.PlayerStarted`))
    (`/Engine/EditorBlueprintResources/StandardMacros.IncrementInt` (`self.TurnNumber`)
      (:`  `
        _)))
  (if (`self.IsPlayersTurn`)
    (`self.EndPlayerTurn`)
    (else
      (`self.BeginPlayerTurn`)))
  (bind _output_get (set `self.IsPlayersTurn` (not (`self.IsPlayersTurn`))))
  (bind _asbp_card_controller (cast `/Game/CardUI/BP_CardController` (`|GetArrayItem` (`/Game/CardUI/BP_CardGameMode.PlayerControllers` (`self.GameMode`)))))
  (message `/Game/CardUI/BPI_PlayerUI.UpdateTurnUI` (`/Game/CardUI/BP_CardController.CardHUD` _asbp_card_controller) _output_get (`self.TurnNumber`)))

(event `Attack`
  (params (AttackingCard :type "/Game/CardUI/BP_CardInstance Object Reference") (TargetedCard :type "/Game/CardUI/BP_CardInstance Object Reference"))
  (if (`KismetStringLibrary.EqualEqual_StrStr` (`KismetSystemLibrary.GetDisplayName` (`self.GetOwner` TargetedCard)) (`KismetSystemLibrary.GetDisplayName` (`self.GetOwner` AttackingCard)))
    (`KismetSystemLibrary.PrintString` "Attacking Own Card")
    (else
      (set `self.Temp_AttackingCardDamage` (`/Game/CardUI/BP_CardInstance.CurrentAttack` AttackingCard))
      (set `self.Temp_TargetedCardDamage` (`/Game/CardUI/BP_CardInstance.CurrentHealth` TargetedCard))
      (`/Game/CardUI/BP_CardInstance.InteractWithOtherCard` TargetedCard (`self.Temp_AttackingCardDamage`))
      (`/Game/CardUI/BP_CardInstance.InteractWithOtherCard` AttackingCard (`self.Temp_TargetedCardDamage`)))))

(event `CardPlacementRequest`
  (params (NewParam :type Boolean)))

(event `BeginGame`
  (bind _playercontrollers (`/Game/CardUI/BP_CardGameMode.PlayerControllers` (`self.GameMode`)))
  (bind _output_get (set `self.IsPlayersTurn` (`KismetMathLibrary.RandomBool`)))
  (set `self.PlayerStarted` _output_get)
  (for _array_element _playercontrollers
    (for _ (range 1 (+ (`/Game/CardUI/BP_CardGameMode.StartingHandSize` (`self.GameMode`)) 1))
      (message `/Game/CardUI/BPI_CardController.DrawCard` _array_element)))
  (if _output_get
    (`self.BeginPlayerTurn`)
    (else
      (`self.EndPlayerTurn`)))
  (bind _asbp_card_controller (cast `/Game/CardUI/BP_CardController` (`|GetArrayItem` _playercontrollers)))
  (message `/Game/CardUI/BPI_PlayerUI.UpdateTurnUI` (`/Game/CardUI/BP_CardController.CardHUD` _asbp_card_controller) (`self.IsPlayersTurn`) (`self.TurnNumber`)))

(fn `BeginPlayerTurn`
  (bind _playercontrollers (`/Game/CardUI/BP_CardGameMode.PlayerControllers` (`self.GameMode`)))
  (message `/Game/CardUI/BPI_CardController.EndTurn` (`|GetArrayItem` _playercontrollers 1))
  (message `/Game/CardUI/BPI_CardController.StartTurn` (`|GetArrayItem` _playercontrollers)))

(fn `EndPlayerTurn`
  (bind _playercontrollers (`/Game/CardUI/BP_CardGameMode.PlayerControllers` (`self.GameMode`)))
  (message `/Game/CardUI/BPI_CardController.EndTurn` (`|GetArrayItem` _playercontrollers))
  (message `/Game/CardUI/BPI_CardController.StartTurn` (`|GetArrayItem` _playercontrollers 1)))

(fn `UserConstructionScript`)