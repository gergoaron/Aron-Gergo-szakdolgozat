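; BP_HeroInstance is a hero actor in the card UI that shows a portrait and health through a W_Hero widget on its HeroFace component.
; BeginPlay caches the widget, sets its image and health from the actor's max health, and redraws it.
; InteractWithCard subtracts card damage, clamps health at zero and pushes the new value to the widget; the zero-health branch is still empty.
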(event `self.ReceiveBeginPlay`
  (bind _heromaxhealth (`self.HeroMaxHealth`))
  (bind _asw_hero (cast `/Game/CardUI/W_Hero` (`WidgetComponent.GetWidget` (`self.HeroFace`))))
  (set `self.HeroWidgetRef` _asw_hero)
  (set `/Game/CardUI/W_Hero.Image` (`self.HeroImage`) _asw_hero)
  (set `/Game/CardUI/W_Hero.HeroStartingHealth` _heromaxhealth _asw_hero)
  (set `/Game/CardUI/W_Hero.HeroCurrentHealth` _heromaxhealth _asw_hero)
  (`/Game/CardUI/W_Hero.Redraw` _asw_hero)
  (set `self.HeroWidgetRef` _asw_hero)
  (set `self.HeroCurrentHealth` (`self.HeroMaxHealth`)))

(event `InteractWithCard`
  (params (CardDamage :type Integer))
  (bind _herowidgetref (`self.HeroWidgetRef`))
  (bind _output_get (set `self.HeroCurrentHealth` (`KismetMathLibrary.Max` (- (`self.HeroCurrentHealth`) CardDamage))))
  (set `/Game/CardUI/W_Hero.HeroCurrentHealth` _output_get _herowidgetref)
  (`/Game/CardUI/W_Hero.Redraw` _herowidgetref)
  (if (<= (`self.HeroCurrentHealth`) 0)
    _))

(fn `UserConstructionScript`)