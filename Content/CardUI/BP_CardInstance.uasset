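; BP_CardInstance is an in-world card actor that shows its card info on a W_Card widget and tracks health and attack.
; A gated Tick glides it to a destination at constant speed, opened by StartReposition and closed on arrival.
; Combat applies the other card's attack as damage, redraws the face and has CardPlacement destroy it at zero health.
; CanAttack requires remaining attacks, health and attack power.
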(event `self.ReceiveBeginPlay`
  (bind _cardinfo (`self.CardInfo`))
  (bind (_cardname _cardimage _carddescription _backgroundcolor _cardmana _cardattack _cardhealth) (break `/Game/CardUI/S_CardInfo` _cardinfo))
  (bind _asw_card (cast `/Game/CardUI/W_Card` (`WidgetComponent.GetUserWidgetObject` (`self.CardFace`))))
  (set `/Game/CardUI/W_Card.CardInfo` _cardinfo _asw_card)
  (`/Game/CardUI/W_Card.Redraw` _asw_card)
  (set `self.CurrentHealth` _cardhealth)
  (set `self.CurrentAttack` _cardattack)
  (bind _asw_card_2 (cast `/Game/CardUI/W_Card` (`WidgetComponent.GetWidget` (`self.CardFace`))))
  (set `self.CardWidgetRef` _asw_card_2))

(event `self.ReceiveTick`
  (params (DeltaSeconds :type "Float (single-precision)"))
  (bind _returnvalue (`self.K2_GetActorLocation`))
  (`/Engine/EditorBlueprintResources/StandardMacros.Gate` true :!label _label
    (:`Exit`
      (if (== (stale `StartReposition` Destination) _returnvalue)
        (`self.Reposition Complete`)
        (else
          (`self.K2_SetActorLocation` (`KismetMathLibrary.VInterpTo_Constant` _returnvalue (stale `StartReposition` Destination) DeltaSeconds (stale `StartReposition` InterpolationSpeed))))))))

(event `StartReposition`
  (params (Destination :type "Vector Structure") (InterpolationSpeed :type "Float (double-precision)"))
  (goto _label :!via `Open`))

(event `Reposition Complete`
  (goto _label :!via `Close`))

(fn `CanAttack`
  (returns (`Can I Attack` :type Boolean))
  (return (and (> (`self.AttacksRemaining`) 0) (> (`self.CurrentHealth`) 0) (> (`self.CurrentAttack`) 0))))

(fn `HealthDamage`
  (params (Amount :type Integer))
  (bind _output_get (set `self.CurrentHealth` (`KismetMathLibrary.Max` (- (`self.CurrentHealth`) Amount))))
  (setmembers `/Game/CardUI/S_CardInfo` :`StructRef` (`self.CardInfo`) :`CardHealth_Current` _output_get))

(fn `InteractWithOtherCard`
  (params (OtherCardAttack :type Integer))
  (`self.HealthDamage` OtherCardAttack)
  (set `/Game/CardUI/W_Card.CardInfo` (`self.CardInfo`) (`self.CardWidgetRef`))
  (`/Game/CardUI/W_Card.Redraw` (`self.CardWidgetRef`))
  (if (<= (`self.CurrentHealth`) 0)
    (`/Game/CardUI/BP_CardPlacement.DestroyCard` (`self.CardPlacement`) self)))

(fn `UserConstructionScript`)