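; Placement actor that manages a row of card actors in the world, spawning, spacing and removing them.
; PlaceCard spawns an owned BP_CardInstance from card info, stores it in Cards and triggers a reposition of the whole row, which DestroyCard repeats after a delayed removal.
; CalculateCardPosition centers cards along world Y around the actor, stacking them slightly in Z and raising selected ones, while each card interpolates to its slot.
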(event `PlaceCard`
  (params (CardInfo :type "/Game/CardUI/S_CardInfo Structure") (Owner :type "Controller Object Reference"))
  (bind _newlocation (`self.CalculateCardPosition` (`KismetArrayLibrary.Array_Length` (`self.Cards`))))
  (bind _returnvalue (`|SpawnActorFromClass` "/Game/CardUI/BP_CardInstance.BP_CardInstance_C" (`KismetMathLibrary.Conv_VectorToTransform` _newlocation) "Undefined" "MultiplyWithRoot" null CardInfo self null))
  (`self.SetOwner` _returnvalue Owner)
  (`KismetArrayLibrary.Array_Add` (`self.Cards`) _returnvalue)
  (`self.UpdateCardPositions`)
  (`KismetSystemLibrary.PrintString` (`KismetSystemLibrary.GetDisplayName` (`self.GetOwner` _returnvalue))))

(event `UpdateCardPositions`
  (for (_array_element _array_index) (`self.Cards`)
    (bind _newlocation (`self.CalculateCardPosition` _array_index (`/Game/CardUI/BP_CardInstance.IsSelected` _array_element)))
    (`/Game/CardUI/BP_CardInstance.StartReposition` _array_element _newlocation 2500.0)))

(event `DestroyCard`
  (params (Card :type "/Game/CardUI/BP_CardInstance Object Reference"))
  (`KismetSystemLibrary.Delay` 1.0)
  (`KismetArrayLibrary.Array_RemoveItem` (`self.Cards`) Card)
  (`self.K2_DestroyActor` Card)
  (`self.UpdateCardPositions`))

(fn `CalculateCardPosition`
  (params (CardIndex :type Integer) (IsSelected :type Boolean))
  (returns (NewLocation :type "Vector Structure"))
  (return (`KismetMathLibrary.MakeVector` (.x (`self.K2_GetActorLocation`)) (+ (.y (`self.K2_GetActorLocation`)) (* (- (/ (`KismetMathLibrary.Conv_IntToDouble` (`KismetArrayLibrary.Array_Length` (`self.Cards`))) 2.0) (+ (`KismetMathLibrary.Conv_IntToDouble` (`local.CardIndex`)) 0.5)) (`self.CardSpacing`))) (+ (.z (`self.K2_GetActorLocation`)) (* 0.01 (`local.CardIndex`)) (* (`local.IsSelected`) 200)))))

(fn `UserConstructionScript`)